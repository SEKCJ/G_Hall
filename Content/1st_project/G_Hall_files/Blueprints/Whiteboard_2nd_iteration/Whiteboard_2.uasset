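; Whiteboard actor, second iteration, that receives marker hits and shows ink by spawning decal-like mark actors.
; MarkMe checks that the hit component overlaps Box, then spawns a rotated, scaled Marker_color at the hit location with the passed color material.
; EraseMe is an empty stub, with its Marker_color_2 spawning logic left disconnected.
; The Status debug print never fires here, since this graph only sets Status false.
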(event EventBeginPlay
  (Variables|Default|SetStatus false))

(event Collision|EventActorBeginOverlap
  (params (OtherActor :type Actor%20Object%20Reference)))

(fn ConstructionScript)

(fn MarkMe
  (params (Hit :type Hit%20Result%20Structure) (HitComponent :type Primitive%20Component%20Object%20Reference) (New_Marker_Color :type Material%20Instance%20Object%20Reference) (Overlapping_component :type Actor%20Object%20Reference) (Detected :type Integer))
  (bind _location (Collision|BreakHitResult Hit))
  (Utilities|FlowControl|Sequence
    (:then_0
      ;[1 1 1] Coloring
      (if (Class|PrimitiveComponent|IsOverlappingComponent HitComponent (Variables|Default|GetBox))
        (bind _returnvalue (Game|SpawnActorfromClass "/Game/1st_project/G_Hall_files/Blueprints/Whiteboard_2nd_iteration/Marker_color.Marker_color_C" (Math|Transform|MakeTransform (Math|Vector|MakeVector (.x _location) (.y _location) (.z _location)) "0,0.000000,-90.000000" (Variables|Default|GetSize)) "AlwaysSpawn" 0 New_Marker_Color 0))
        (Rendering|Material|SetMaterial (Variables|/Script/Engine.StaticMeshActor|GetStaticMeshComponent _returnvalue) 0 New_Marker_Color)))
    (:then_1
      (if (Variables|Default|GetStatus)
        (Development|PrintString "Overlap Detected")
        (Variables|Default|SetStatus false)))))

(fn EraseMe
  (params (HitEraser :type Hit%20Result%20Structure) (HitComponentEraser :type Primitive%20Component%20Object%20Reference)))