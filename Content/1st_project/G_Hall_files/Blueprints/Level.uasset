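; Level Blueprint-style actor that switches a physics lab's lighting on and off as something enters or leaves a trigger box.
; BeginPlay gathers the room's point lights and tube fixture meshes into arrays.
; Box overlap begin shows the lights and swaps wall, tube, ceiling and floor materials to one set of instances; overlap end hides them and applies the alternate set, so surface appearance follows the light state.
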(event OnComponentEndOverlap(Box)
  (params (OverlappedComponent :type Primitive%20Component%20Object%20Reference) (OtherActor :type Actor%20Object%20Reference) (OtherComp :type Primitive%20Component%20Object%20Reference) (OtherBodyIndex :type Integer))
  (Rendering|SetVisibility (stale EventBeginPlay _output_get) false false)
  (Rendering|Material|SetMaterial (Variables|Default|GetPhysics_lab) 0 "/Game/1st_project/G_Hall_files/Materials/Wall_materials/Painted_Cinder_Blocks_MAT_Inst1.Painted_Cinder_Blocks_MAT_Inst1")
  (Rendering|Material|SetMaterial (Utilities|Array|MakeArray (Variables|Default|GetLightsFixed) (Variables|Default|GetLightsFixed1) (Variables|Default|GetLightsFixed2) (Variables|Default|GetLightsFixed3) (Variables|Default|GetLightsFixed4) (Variables|Default|GetLightsFixed5) (Variables|Default|GetLightsFixed6) (Variables|Default|GetLightsFixed7) (Variables|Default|GetLightsFixed8) (Variables|Default|GetLightsFixed9) (Variables|Default|GetLightsFixed10) (Variables|Default|GetLightsFixed11)) 0 "/Game/1st_project/DemoRoom/Materials/M_LightTube_Inst1.M_LightTube_Inst1")
  (Rendering|Material|SetMaterial (Variables|Default|GetCeiling) 3 "/Game/1st_project/G_Hall_files/Meshes/Ceiling/Tile_main_M_Inst.Tile_main_M_Inst")
  (Rendering|Material|SetMaterial (Variables|Default|GetFloor) 0 "/Game/1st_project/G_Hall_files/Materials/TileFloor_Inst2.TileFloor_Inst2"))

(event OnComponentBeginOverlap(Box)
  (params (OverlappedComponent :type Primitive%20Component%20Object%20Reference) (OtherActor :type Actor%20Object%20Reference) (OtherComp :type Primitive%20Component%20Object%20Reference) (OtherBodyIndex :type Integer) (bFromSweep :type Boolean) (SweepResult :type Hit%20Result%20Structure%20%28by%20ref%29))
  (Rendering|SetVisibility (stale EventBeginPlay _output_get) true false)
  (Rendering|Material|SetMaterial (Variables|Default|GetPhysics_lab) 0 "/Game/1st_project/G_Hall_files/Materials/Wall_materials/Painted_Cinder_Blocks_MAT_Inst.Painted_Cinder_Blocks_MAT_Inst")
  (Rendering|Material|SetMaterial (Utilities|Array|MakeArray (Variables|Default|GetLightsFixed) (Variables|Default|GetLightsFixed1) (Variables|Default|GetLightsFixed2) (Variables|Default|GetLightsFixed3) (Variables|Default|GetLightsFixed4) (Variables|Default|GetLightsFixed5) (Variables|Default|GetLightsFixed6) (Variables|Default|GetLightsFixed7) (Variables|Default|GetLightsFixed8) (Variables|Default|GetLightsFixed9) (Variables|Default|GetLightsFixed10) (Variables|Default|GetLightsFixed11)) 0 "/Game/1st_project/DemoRoom/Materials/M_LightTube_Inst.M_LightTube_Inst")
  (Rendering|Material|SetMaterial (Variables|Default|GetCeiling) 3 "/Game/1st_project/G_Hall_files/Meshes/Ceiling/Tile_Inst.Tile_Inst")
  (Rendering|Material|SetMaterial (Variables|Default|GetFloor) 0 "/Game/1st_project/G_Hall_files/Materials/TileFloor_Inst1.TileFloor_Inst1"))

(event EventBeginPlay
  (bind _output_get (Variables|Default|Set1st_group_of_lights (Utilities|Array|MakeArray (Variables|Default|GetPointLight) (Variables|Default|GetPointLight1) (Variables|Default|GetPointLight2) (Variables|Default|GetPointLight3) (Variables|Default|GetPointLight4) (Variables|Default|GetPointLight5) (Variables|Default|GetPointLight6) (Variables|Default|GetPointLight7) (Variables|Default|GetPointLight16))))
  (Variables|Default|SetGroup_of_light_meshes (Utilities|Array|MakeArray (Variables|Default|GetLightsFixed) (Variables|Default|GetLightsFixed1) (Variables|Default|GetLightsFixed2) (Variables|Default|GetLightsFixed3) (Variables|Default|GetLightsFixed4) (Variables|Default|GetLightsFixed5) (Variables|Default|GetLightsFixed6) (Variables|Default|GetLightsFixed7) (Variables|Default|GetLightsFixed8) (Variables|Default|GetLightsFixed9) (Variables|Default|GetLightsFixed10) (Variables|Default|GetLightsFixed11))))

(fn ConstructionScript)