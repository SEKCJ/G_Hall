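; BP_Pickup is a grippable VR pickup actor that implements motion-controller grip interface functions.
; Grip and release events track the holding controller and a held flag, which IsHeld reports back.
; The other functions return fixed grip settings: client-side movement, simulation on drop, no secondary grip or socketing.
; GetPrimaryGripType leaves its InteractiveCollisionWithPhysics return unconnected, so that value is never returned.
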(event EventBeginPlay)

(event Collision|EventActorBeginOverlap
  (params (OtherActor :type Actor%20Object%20Reference)))

(event EventOnGrip
  (params (GrippingController :type Grip%20Motion%20Controller%20Component%20Object%20Reference) (GripInformation :type BP%20Actor%20Grip%20Information%20Structure%20%28by%20ref%29))
  (Variables|Default|SetGrippingController GrippingController)
  (Variables|Default|SetGripped true))

(event EventOnGripRelease
  (params (ReleasingController :type Grip%20Motion%20Controller%20Component%20Object%20Reference) (GripInformation :type BP%20Actor%20Grip%20Information%20Structure%20%28by%20ref%29) (bWasSocketed :type Boolean))
  (Variables|Default|SetGrippingController 0)
  (Variables|Default|SetGripped false))

(fn ConstructionScript)

(fn AdvancedGripSettings
  (return ""))

(fn ClosestGripSlotinRange
  (params (WorldLocation :type Vector :default "0, 0, 0") (bSecondarySlot :type Boolean) (CallingController :type Grip%20Motion%20Controller%20Component%20Object%20Reference) (OverridePrefix :type Name :default "None"))
  (return false ""))

(fn DenyGripping
  (return false))

(fn GetGripStiffnessandDamping
  (return 1.5e+03 2e+02))

(fn GetPrimaryGripType
  (params (bIsSlot :type Boolean)))

(fn GripBreakDistance
  (return 1e+02))

(fn GripLateUpdateSetting
  (return "NotWhenCollidingOrDoubleGripping"))

(fn GripMovementReplicationType
  (return "ForceClientSideMovement"))

(fn IsHeld
  (return (Variables|Default|GetGrippingController) (Variables|Default|GetGripped)))

(fn RequestsSocketing
  (return 0 "None" "" false))

(fn SecondaryGripType
  (return "SG_None"))

(fn SimulateonDrop
  (return true))

(fn TeleportBehavior
  (return "TeleportAllComponents"))