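; Grippable VR monitor prop that glows when overlapped and can be picked up through grip interface functions.
; On BeginPlay it copies its static mesh into a procedural mesh, scales it and applies a blue glow material as a hidden highlight.
; Overlap toggles the highlight and gripping hides it.
; On release, linear and angular velocities are divided by Momentum, and the grip state is cleared.
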(event OnComponentBeginOverlap(StaticMeshComponent)
  (params (OverlappedComponent :type Primitive%20Component%20Object%20Reference) (OtherActor :type Actor%20Object%20Reference) (OtherComp :type Primitive%20Component%20Object%20Reference) (OtherBodyIndex :type Integer) (bFromSweep :type Boolean) (SweepResult :type Hit%20Result%20Structure%20%28by%20ref%29))
  (Rendering|SetVisibility (Variables|Default|GetProceduralMesh) true false))

(event OnComponentEndOverlap(StaticMeshComponent)
  (params (OverlappedComponent :type Primitive%20Component%20Object%20Reference) (OtherActor :type Actor%20Object%20Reference) (OtherComp :type Primitive%20Component%20Object%20Reference) (OtherBodyIndex :type Integer))
  (Rendering|SetVisibility (Variables|Default|GetProceduralMesh) false false))

(event EventBeginPlay
  (bind _proceduralmesh (Variables|Default|GetProceduralMesh))
  (bind _proceduralmesh_2 (Variables|Default|GetProceduralMesh))
  (bind _returnvalue (Transformation|GetWorldTransform _proceduralmesh))
  ;[1 1 1] Make Glowing Mesh
  (Class|KismetProceduralMeshLibrary|CopyProceduralMeshfromStaticMeshComponent (Variables|Debug|GetStaticMeshComponent) 0 _proceduralmesh false)
  (Transformation|SetWorldTransform _proceduralmesh (Math|Transform|MakeTransform (.location _returnvalue) (.rotation _returnvalue) (* (.scale _returnvalue) (Variables|Default|GetScale))) false false)
  (for _index (range 0 (Rendering|Material|GetNumMaterials (Variables|Debug|GetStaticMeshComponent)))
    (Rendering|Material|SetMaterial _proceduralmesh_2 _index "/Game/1st_project/G_Hall_files/Materials/BlueGlow_Inst_Inst_Inst.BlueGlow_Inst_Inst_Inst")
    (Rendering|SetVisibility _proceduralmesh_2 false false)))

(event EventOnGripRelease
  (params (ReleasingController :type Grip%20Motion%20Controller%20Component%20Object%20Reference) (GripInformation :type BP%20Actor%20Grip%20Information%20Structure%20%28by%20ref%29) (bWasSocketed :type Boolean))
  (bind _momentum (Variables|Default|GetMomentum))
  (bind _staticmeshcomponent (Variables|Debug|GetStaticMeshComponent))
  (bind _returnvalue (Physics|GetPhysicsLinearVelocity _staticmeshcomponent "None"))
  (Physics|SetPhysicsLinearVelocity _staticmeshcomponent (/ _returnvalue _momentum) false "None")
  (bind _returnvalue_2 (Class|PrimitiveComponent|GetPhysicsAngularVelocityinRadians _staticmeshcomponent "None"))
  (Class|PrimitiveComponent|SetPhysicsAngularVelocityinRadians _staticmeshcomponent (/ _returnvalue_2 _momentum) false "None")
  (Variables|Default|SetGrippingController 0)
  (Variables|Default|SetGripped false))

(event EventOnGrip
  (params (GrippingController :type Grip%20Motion%20Controller%20Component%20Object%20Reference) (GripInformation :type BP%20Actor%20Grip%20Information%20Structure%20%28by%20ref%29))
  (Variables|Default|SetGrippingController GrippingController)
  (Variables|Default|SetGripped true)
  (Rendering|SetVisibility (Variables|Default|GetProceduralMesh) false false))

(fn ConstructionScript)

(fn AdvancedGripSettings
  (return ""))

(fn ClosestGripSlotinRange
  (params (WorldLocation :type Vector :default "0, 0, 0") (bSecondarySlot :type Boolean) (CallingController :type Grip%20Motion%20Controller%20Component%20Object%20Reference) (OverridePrefix :type Name :default "None"))
  (return false ""))

(fn DenyGripping
  (return false))

(fn GetGripStiffnessandDamping
  (return 1.5e+03 2e+02))

(fn GetPrimaryGripType
  (params (bIsSlot :type Boolean)))

(fn GripBreakDistance
  (return 1e+02))

(fn GripLateUpdateSetting
  (return "NotWhenCollidingOrDoubleGripping"))

(fn GripMovementReplicationType
  (return "ForceClientSideMovement"))

(fn IsHeld
  (return (Variables|Default|GetGrippingController) (Variables|Default|GetGripped)))

(fn RequestsSocketing
  (return 0 "None" "" false))

(fn SecondaryGripType
  (return "SG_None"))

(fn SimulateonDrop
  (return true))

(fn TeleportBehavior
  (return "TeleportAllComponents"))