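; Grippable VR axe that slices SlicingTable actors when its edge hits them while activated.
; Using the axe toggles the active state and a material glow.
; Tip and main edge hits pass the contact and a rolling-average velocity, sampled on Tick while gripped, to the table's SliceMe.
; An FPS_VivePawnCharacter grip skips enabling Tick and sets IgnoreVelocity, since swing speed and angle are hard to achieve in 2D.
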(event OnComponentHit(StaticMeshComponent)
  (params (HitComponent :type Primitive%20Component%20Object%20Reference) (OtherActor :type Actor%20Object%20Reference) (OtherComp :type Primitive%20Component%20Object%20Reference) (NormalImpulse :type Vector :default "0, 0, 0") (Hit :type Hit%20Result%20Structure%20%28by%20ref%29))
  (Variables|Default|SetHitComp HitComponent)
  (Variables|Default|SetOthercomp OtherComp))

(event OnComponentHit(SwordEdgeTip)
  (params (HitComponent :type Primitive%20Component%20Object%20Reference) (OtherActor :type Actor%20Object%20Reference) (OtherComp :type Primitive%20Component%20Object%20Reference) (NormalImpulse :type Vector :default "0, 0, 0") (Hit :type Hit%20Result%20Structure%20%28by%20ref%29))
  (if (Variables|Default|GetbIsActive)
    (bind _asslicing_table (Utilities|Casting|CastToSlicingTable OtherActor))
    (Default|SliceMe _asslicing_table Hit HitComponent OtherComp (Variables|Default|GetVelocityAverage) (Variables|Default|GetIgnoreVelocity))))

(event OnComponentHit(SwordEdgeMain)
  (params (HitComponent :type Primitive%20Component%20Object%20Reference) (OtherActor :type Actor%20Object%20Reference) (OtherComp :type Primitive%20Component%20Object%20Reference) (NormalImpulse :type Vector :default "0, 0, 0") (Hit :type Hit%20Result%20Structure%20%28by%20ref%29))
  (if (Variables|Default|GetbIsActive)
    (bind _asslicing_table (Utilities|Casting|CastToSlicingTable OtherActor))
    (Default|SliceMe _asslicing_table Hit HitComponent OtherComp (Variables|Default|GetVelocityAverage) (Variables|Default|GetIgnoreVelocity))))

(event EventBeginPlay
  (bind _returnvalue (Rendering|Material|CreateDynamicMaterialInstance (Variables|Default|GetStaticMeshComponent) 3 "/Game/VRExpansion/Vive/Testing/Slicer/01_-_Defaultg.01_-_Defaultg" :!class /Script/Engine.PrimitiveComponent))
  (bind _output_get (Variables|Default|SetDynamicMat _returnvalue))
  (Rendering|Material|SetScalarParameterValue _output_get "GlowScaler" 0.0 :!class /Script/Engine.MaterialInstanceDynamic))

(event Collision|EventActorBeginOverlap
  (params (OtherActor :type Actor%20Object%20Reference)))

(event EventOnUsed
  (Variables|Default|SetbIsActive true)
  (Rendering|Material|SetScalarParameterValue (Variables|Default|GetDynamicMat) "GlowScaler" 8e+02 :!class /Script/Engine.MaterialInstanceDynamic))

(event EventOnGripRelease
  (params (ReleasingController :type Grip%20Motion%20Controller%20Component%20Object%20Reference) (GripInformation :type BP%20Actor%20Grip%20Information%20Structure%20%28by%20ref%29))
  (Actor|Tick|SetActorTickEnabled false))

(event EventTick
  (params (DeltaSeconds :type Float%20%28single-precision%29))
  (Variables|Default|SetVelocityAverage (Class|VRExpansionFunctionLibrary|LowPassFilterRollingAverage (Variables|Default|GetVelocityAverage) (Transformation|GetVelocity) 2)))

(event EventOnGrip
  (params (GrippingController :type Grip%20Motion%20Controller%20Component%20Object%20Reference) (GripInformation :type BP%20Actor%20Grip%20Information%20Structure%20%28by%20ref%29))
  (Utilities|Casting|CastToFPS_VivePawnCharacter (Components|GetOwner GrippingController)
    (:then
      (Variables|Default|SetIgnoreVelocity true) ; Hard to hit the required swing speed and angle in 2D
    )
    (:CastFailed
      (Actor|Tick|SetActorTickEnabled true)
      (if (.bIsSlotGrip (Utilities|Struct|BreakBPActorGripInformation GripInformation))
        _))))

(event EventOnEndUsed
  (Variables|Default|SetbIsActive false)
  (Rendering|Material|SetScalarParameterValue (Variables|Default|GetDynamicMat) "GlowScaler" 0.0 :!class /Script/Engine.MaterialInstanceDynamic))

(fn ConstructionScript)