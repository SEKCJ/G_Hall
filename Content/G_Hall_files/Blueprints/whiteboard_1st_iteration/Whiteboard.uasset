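; Whiteboard actor Blueprint, a first-iteration board that can be drawn on with decals.
; MarkMe takes a hit result and spawns a black plastic decal at the hit location.
; BeginPlay caches the static mesh's world transform, but the logic to restore it is disconnected.
; The component hit event is empty, so marks appear only when MarkMe is called.
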(event OnComponentHit(StaticMesh)
  (params (HitComponent :type Primitive%20Component%20Object%20Reference) (OtherActor :type Actor%20Object%20Reference) (OtherComp :type Primitive%20Component%20Object%20Reference) (NormalImpulse :type Vector :default "0, 0, 0") (Hit :type Hit%20Result%20Structure%20%28by%20ref%29)))

(event EventBeginPlay
  (Variables|Default|SetInitial_transform (Transformation|GetWorldTransform (Variables|Default|GetStaticMesh))))

(event Collision|EventActorBeginOverlap
  (params (OtherActor :type Actor%20Object%20Reference)))

(fn ConstructionScript)

(fn MarkMe
  (params (Hit :type Hit%20Result%20Structure))
  (bind _returnvalue (Rendering|Decal|SpawnDecalatLocation "/Game/G_Hall_files/Models/Table_conn/Black_Plastic.Black_Plastic" (Variables|Default|GetSize) (.Location (Collision|BreakHitResult Hit)) "-90.000000,0.000000,0.000000" 0.0)))