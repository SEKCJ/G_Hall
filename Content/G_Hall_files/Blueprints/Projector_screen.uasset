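; Projector screen actor that stretches as its holding point moves vertically, implementing a VR grip interface.
; BeginPlay caches the absolute world height of HoldingPoint and the Z scale of the Sphere component.
; Tick, behind a short Delay, adds HoldingPoint's normalized height change, divided by Equalizer, to that base Z scale.
; Grip interface functions return fixed values, allowing gripping with physics-based interactive collision.
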(event EventTick
  (params (DeltaSeconds :type Float%20%28single-precision%29))
  (bind _sphere (Variables|Default|GetSphere))
  (bind _initial_position (Variables|Default|GetInitial_position))
  (bind _returnvalue (Transformation|GetWorldTransform _sphere))
  (Utilities|FlowControl|Delay 0.01)
  (Transformation|SetWorldTransform (Variables|Default|GetSphere) (Math|Transform|MakeTransform (.location _returnvalue) (.rotation _returnvalue) (Math|Vector|MakeVector (.x (.scale _returnvalue)) (.y (.scale _returnvalue)) (+ (/ (/ (- _initial_position (.z (.location (Transformation|GetWorldTransform (Variables|Default|GetHoldingPoint))))) _initial_position) (Variables|Default|GetEqualizer)) (Variables|Default|GetInitial_scale)))) false false))

(event EventBeginPlay
  (Variables|Default|SetInitial_position (Math|Float|Absolute(Float) (.z (.location (Transformation|GetWorldTransform (Variables|Default|GetHoldingPoint))))))
  (Variables|Default|SetInitial_scale (.z (.scale (Transformation|GetWorldTransform (Variables|Default|GetSphere))))))

(fn ConstructionScript)

(fn AdvancedGripSettings
  (return ""))

(fn ClosestGripSlotinRange
  (params (WorldLocation :type Vector :default "0, 0, 0") (bSecondarySlot :type Boolean) (CallingController :type Grip%20Motion%20Controller%20Component%20Object%20Reference) (OverridePrefix :type Name :default "None"))
  (return false ""))

(fn DenyGripping
  (return false))

(fn GetGripStiffnessandDamping
  (return 0.0 0.0))

(fn GetInteractionSettings
  (return ""))

(fn GetPrimaryGripType
  (params (bIsSlot :type Boolean))
  (return "InteractiveCollisionWithPhysics"))

(fn GripBreakDistance
  (return 0.0))

(fn GripLateUpdateSetting
  (return "LateUpdatesAlwaysOn"))

(fn GripMovementReplicationType
  (return "KeepOriginalMovement"))

(fn IsHeld
  (return 0 false))

(fn IsInteractible
  (return false))

(fn SecondaryGripType
  (return "SG_None"))

(fn SimulateonDrop
  (return false))

(fn TeleportBehavior
  (return "TeleportAllComponents"))