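; Replicated physics door for VR, with a grippable child actor and the door as root for replication.
; BeginPlay detaches the child actor in world space so it does not swing with the door.
; On grip, the server enables door physics and ignores Pawn collision.
; On release, the DoorStop timeline polls door velocity, then disables physics and restores Pawn blocking once the door is still.
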(event Custom|SetCollision
  (params (Collide :type Boolean))
  (bind _door (Variables|Default|GetDoor))
  (if Collide
    (Collision|SetCollisionResponsetoChannel _door "ECC_Pawn" "ECR_Block")
    (else
      (Collision|SetCollisionResponsetoChannel _door "ECC_Pawn" "ECR_Ignore"))))

(event Custom|SetPlayerCollision
  (params (Collide :type Boolean) (Simulation :type Boolean))
  (Physics|SetSimulatePhysics (Variables|Default|GetDoor) Simulation)
  (CallFunction|SetCollision Collide))

(event EventBeginPlay
  (Networking|SwitchHasAuthority
    (:Authority
      _)
    (:Remote
      _))
  (Transformation|DetachFromActor (Variables|/Script/Engine.ChildActorComponent|GetChildActor (Variables|Default|GetChildActor)) "KeepWorld" "KeepWorld" "KeepWorld") ; This is because otherwise it will swing with the door\nCan do this with two totally seperate actors instead but I wanted it all in one blueprint for now\n\nThe door has to be root now because otherwise it doesn't replicate
)

(event Collision|EventActorBeginOverlap
  (params (OtherActor :type Actor%20Object%20Reference)))

(event EventOnChildGrip
  (params (GrippingController :type Grip%20Motion%20Controller%20Component%20Object%20Reference) (GripInformation :type BP%20Actor%20Grip%20Information%20Structure%20%28by%20ref%29))
  (Networking|SwitchHasAuthority
    (:Authority
      (CallFunction|SetPlayerCollision false true)
      (Variables|Default|SetGripped true))))

(event EventOnChildGripRelease
  (params (ReleasingController :type Grip%20Motion%20Controller%20Component%20Object%20Reference) (GripInformation :type BP%20Actor%20Grip%20Information%20Structure%20%28by%20ref%29))
  (Networking|SwitchHasAuthority
    (:Authority
      (Timeline|DoorStop PlayFromStart
        (:Update
          (if (Math|Vector|Equal(Vector) (Transformation|GetComponentVelocity (Variables|Default|GetDoor)) "0, 0, 0" 0.0001)
            (CallFunction|SetPlayerCollision true false)
            (Timeline|DoorStop Stop)))
        (:Finished
          (Variables|Default|SetGripped false))))))

(fn ConstructionScript)

(fn AdvancedGripSettings
  (return ""))

(fn ClosestGripSlotinRange
  (params (WorldLocation :type Vector :default "0, 0, 0") (bSecondarySlot :type Boolean) (CallingController :type Grip%20Motion%20Controller%20Component%20Object%20Reference) (OverridePrefix :type Name :default "None"))
  (return false ""))

(fn DenyGripping
  (return true))

(fn GetGripStiffnessandDamping
  (return 0.0 0.0))

(fn GetInteractionSettings
  (return ""))

(fn GetPrimaryGripType
  (params (bIsSlot :type Boolean))
  (return "InteractiveCollisionWithPhysics"))

(fn GripBreakDistance
  (return 0.0))

(fn GripLateUpdateSetting
  (return "LateUpdatesAlwaysOn"))

(fn GripMovementReplicationType
  (return "KeepOriginalMovement"))

(fn IsHeld
  (return 0 false))

(fn IsInteractible
  (return false))

(fn SecondaryGripType
  (return "SG_None"))

(fn SimulateonDrop
  (return false))

(fn TeleportBehavior
  (return "TeleportAllComponents"))