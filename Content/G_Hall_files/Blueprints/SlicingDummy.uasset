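; SlicingDummy is a target actor that can be repeatedly cut apart by a slicing component.
; On BeginPlay it copies its static mesh into a procedural mesh with collision, then destroys the original.
; SliceMe gates cuts by cooldown, impact angle and blade-plane velocity (optionally ignored), then slices along the hitting component's right vector with a cap.
; Pieces simulate physics, except a still-large main body, and negligibly small ones are destroyed.
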(event EventBeginPlay
  (bind _staticmesh (Variables|Default|GetStaticMesh))
  (Class|KismetProceduralMeshLibrary|CopyProceduralMeshfromStaticMeshComponent _staticmesh 0 (Variables|Default|GetProceduralMesh) true)
  (Development|SetHiddeninGame _staticmesh true false)
  (Collision|SetCollisionEnabled _staticmesh "NoCollision")
  (Components|DestroyComponent _staticmesh))

(event Collision|EventActorBeginOverlap
  (params (OtherActor :type Actor%20Object%20Reference)))

(event EventTick
  (params (DeltaSeconds :type Float%20%28single-precision%29)))

(fn ConstructionScript)

(fn SliceMe
  (params (Hit :type Hit%20Result%20Structure) (HittingComp :type Primitive%20Component%20Object%20Reference) (HitComp :type Primitive%20Component%20Object%20Reference) (Velocity :type Vector) (IgnoreVelocity :type Boolean))
  (bind (_bblockinghit _binitialoverlap _time _distance _location _impactpoint _normal _impactnormal) (Collision|BreakHitResult Hit))
  (bind _returnvalue (Math|Vector|GetRightVector HittingComp))
  (bind _proceduralmesh (Variables|Default|GetProceduralMesh))
  (if (> (Math|Timespan|GetTotalSeconds (- (Math|DateTime|Now) (Variables|Default|GetLastSliceTime))) (Variables|Default|GetSlicingDelay))
    (bind _asprocedural_mesh_component (Utilities|Casting|CastToProceduralMeshComponent HitComp))
    (if (and (< (Math|Vector|DotProduct (Math|Vector|GetForwardVector HittingComp) _impactnormal) (Variables|Default|GetAcceptableDotOfImpact)) (or (> (Math|Vector|VectorLengthSquared (Math|Vector|ProjectVectorontoPlane Velocity _returnvalue)) (Math|Float|Square (Variables|Default|GetRequiredVelocityMagnitudeForSlice))) IgnoreVelocity)) ; Check angle of impact
      (bind _outotherhalfprocmesh (Class|KismetProceduralMeshLibrary|SliceProceduralMesh _asprocedural_mesh_component _location _returnvalue true "CreateNewSectionForCap" "/Game/VRExpansion/Vive/Testing/Button/Button_Mat_Inst.Button_Mat_Inst"))
      (Collision|SetCollisionResponsetoChannel _outotherhalfprocmesh "ECC_Pawn" "ECR_Ignore")
      (if (> (Math|Float|Truncate (.SphereRadius (Collision|GetComponentBounds _asprocedural_mesh_component))) 0)
        (Utilities|IsValid _proceduralmesh
          (:Is%20Valid
            (if (and (== _asprocedural_mesh_component _proceduralmesh) (> (Math|Float|Truncate (.SphereRadius (Collision|GetComponentBounds _asprocedural_mesh_component))) 100))
              _
              (else
                (Physics|SetSimulatePhysics _asprocedural_mesh_component true :!label _label))))
          (:Is%20Not%20Valid
            (goto _label)))
        (else
          (Components|DestroyComponent _asprocedural_mesh_component)))
      (if (> (Math|Float|Truncate (.SphereRadius (Collision|GetComponentBounds _outotherhalfprocmesh))) 0)
        (Physics|SetSimulatePhysics _outotherhalfprocmesh true)
        (else
          (Components|DestroyComponent _outotherhalfprocmesh)))
      (Variables|Default|SetLastSliceTime (Math|DateTime|Now)))))