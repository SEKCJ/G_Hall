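; BP_Locked is a demo-room status label that shows whether a linked actor is locked.
; On Tick, through a short Delay, it casts LinkedTo to BP_Slot_Essential, falling back to BP_InteractableActor_Essential, and reads its Locked flag.
; It sets its TextRender to red "Locked" or green "Unlocked" to match.
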(event EventTick
  (params (DeltaSeconds :type Float%20%28single-precision%29))
  ;[1 1 1] Comment
  (Utilities|FlowControl|Delay 0.2)
  (bind _asbp_slot_essential (Utilities|Casting|CastToBP_Slot_Essential (Variables|Default|GetLinkedTo))
    (:then
      (if (Variables|/Game/1st_project/Essential_Kit/VR_Essential_Kit/Blueprints/BP_Slot_Essential.BP_Slot_Essential_C|GetLocked _asbp_slot_essential)
        (Rendering|Components|TextRender|SetText (Variables|Default|GetTextRender) (Utilities|Text|ToText(String) "Locked") :!label _label)
        (Rendering|Components|TextRender|SetTextRenderColor (Variables|Default|GetTextRender) (Math|Color|MakeColor 0 0 255 255))
        (else
          (Rendering|Components|TextRender|SetText (Variables|Default|GetTextRender) (Utilities|Text|ToText(String) "Unlocked") :!label _label_2)
          (Rendering|Components|TextRender|SetTextRenderColor (Variables|Default|GetTextRender) (Math|Color|MakeColor 0 255 0 255)))))
    (:CastFailed
      (bind _asbp_interactable_actor_essential (Utilities|Casting|CastToBP_InteractableActor_Essential (Variables|Default|GetLinkedTo)))
      (if (Variables|/Game/1st_project/Essential_Kit/VR_Essential_Kit/Blueprints/BP_InteractableActor_Essential.BP_InteractableActor_Essential_C|GetLocked _asbp_interactable_actor_essential)
        (goto _label)
        (else
          (goto _label_2))))))

(fn ConstructionScript)