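; BP_Position is a demo room readout that displays the movement of a linked BP_InteractableActor_Essential through a TextRender.
; On BeginPlay it records the linked actor mesh's world Y as the initial location.
; Every Tick it branches on the actor's Type, showing either the rounded cumulative angle for rotation or the rounded Y offset from the start for translation.
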(event EventTick
  (params (DeltaSeconds :type Float%20%28single-precision%29))
  ;[1 1 1] Comment
  (bind _asbp_interactable_actor_essential (Utilities|Casting|CastToBP_InteractableActor_Essential (Variables|Default|GetLinkedTo)))
  (switch Utilities|FlowControl|Switch|SwitchonENUM_InteractableActorType_Essetntial (Variables|/Game/1st_project/Essential_Kit/VR_Essential_Kit/Blueprints/BP_InteractableActor_Essential.BP_InteractableActor_Essential_C|GetType _asbp_interactable_actor_essential)
    (:NewEnumerator0
      (Rendering|Components|TextRender|SetText (Variables|Default|GetTextRender) (Utilities|Text|ToText(String) (Utilities|String|Append "Angle : " (Utilities|String|ToString(Integer) (Math|Float|Round (Variables|/Game/1st_project/Essential_Kit/VR_Essential_Kit/Blueprints/BP_InteractableActor_Essential.BP_InteractableActor_Essential_C|GetCumulativeAngle _asbp_interactable_actor_essential)))))))
    (:NewEnumerator1
      (Rendering|Components|TextRender|SetText (Variables|Default|GetTextRender) (Utilities|Text|ToText(String) (Utilities|String|Append "Distance : " (Utilities|String|ToString(Integer) (Math|Float|Round (- (.y (Transformation|GetWorldLocation (Variables|/Game/1st_project/Essential_Kit/VR_Essential_Kit/Blueprints/BP_InteractableActor_Essential.BP_InteractableActor_Essential_C|GetMesh _asbp_interactable_actor_essential))) (Variables|Default|GetInitialLocation))))))))))

(event EventBeginPlay
  ;[1 1 1] Comment
  (bind _asbp_interactable_actor_essential (Utilities|Casting|CastToBP_InteractableActor_Essential (Variables|Default|GetLinkedTo)))
  (Variables|Default|SetInitialLocation (.y (Transformation|GetWorldLocation (Variables|/Game/1st_project/Essential_Kit/VR_Essential_Kit/Blueprints/BP_InteractableActor_Essential.BP_InteractableActor_Essential_C|GetMesh _asbp_interactable_actor_essential)))))

(fn ConstructionScript)