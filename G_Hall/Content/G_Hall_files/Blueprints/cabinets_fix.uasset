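; VR cabinet with two physics doors that stop at trigger boxes, implementing the grip interface but denying gripping on the actor itself.
; Box overlaps zero an unheld door's spin and angular velocity cap; held doors or ending overlaps restore the cap.
; Box2 records the overlapping component's Z angular speed, which picks a soft or loud sound when unheld Door2 stops.
; Door has no sound.
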(event OnComponentEndOverlap(Box)
  (params (OverlappedComponent :type Primitive%20Component%20Object%20Reference) (OtherActor :type Actor%20Object%20Reference) (OtherComp :type Primitive%20Component%20Object%20Reference) (OtherBodyIndex :type Integer))
  (bind _door2 (Variables|Default|GetDoor2))
  ;[1 1 1] Comment
  (Class|GrippableStaticMeshComponent|SimulateonDrop _door2)
  (Class|PrimitiveComponent|SetPhysicsMaxAngularVelocityinRadians _door2 1.570796 false "None"))

(event OnComponentEndOverlap(Box1)
  (params (OverlappedComponent :type Primitive%20Component%20Object%20Reference) (OtherActor :type Actor%20Object%20Reference) (OtherComp :type Primitive%20Component%20Object%20Reference) (OtherBodyIndex :type Integer))
  (bind _door (Variables|Default|GetDoor))
  ;[1 1 1] Comment
  (Class|GrippableStaticMeshComponent|SimulateonDrop _door)
  (Class|PrimitiveComponent|SetPhysicsMaxAngularVelocityinRadians _door 1.570796 false "None"))

(event OnComponentBeginOverlap(Box2)
  (params (OverlappedComponent :type Primitive%20Component%20Object%20Reference) (OtherActor :type Actor%20Object%20Reference) (OtherComp :type Primitive%20Component%20Object%20Reference) (OtherBodyIndex :type Integer) (bFromSweep :type Boolean) (SweepResult :type Hit%20Result%20Structure%20%28by%20ref%29))
  (bind _returnvalue (Physics|GetPhysicsAngularVelocityinDegrees OtherComp "None"))
  (Variables|Default|SetAngular_speed (Math|Float|Absolute(Float) (.z _returnvalue))))

(event OnComponentBeginOverlap(Box)
  (params (OverlappedComponent :type Primitive%20Component%20Object%20Reference) (OtherActor :type Actor%20Object%20Reference) (OtherComp :type Primitive%20Component%20Object%20Reference) (OtherBodyIndex :type Integer) (bFromSweep :type Boolean) (SweepResult :type Hit%20Result%20Structure%20%28by%20ref%29))
  (bind _door2 (Variables|Default|GetDoor2))
  (bind _box (Variables|Default|GetBox))
  (bind _returnvalue (Transformation|GetWorldTransform _box))
  ;[1 1 1] Comment
  (bind _bisheld (Class|GrippableStaticMeshComponent|IsHeld _door2))
  (if _bisheld
    (Class|PrimitiveComponent|SetPhysicsMaxAngularVelocityinRadians _door2 1.570796 false "None")
    (Class|GrippableStaticMeshComponent|SimulateonDrop _door2)
    (else
      (Class|PrimitiveComponent|SetPhysicsAngularVelocityinDegrees _door2 "0, 0, 0" false "None")
      (Class|PrimitiveComponent|SetPhysicsMaxAngularVelocityinRadians _door2 0.0 false "None")
      (Class|GrippableStaticMeshComponent|SimulateonDrop _door2)
      (if (<= (Variables|Default|GetAngular_speed) (Variables|Default|Getnoise_threshold))
        (Audio|PlaySoundatLocation "/Game/G_Hall_files/Blueprints/soft_cabinet_door.soft_cabinet_door" (.location _returnvalue) (.rotation _returnvalue) 1.0 1.0 0.0 0 0 0)
        (else
          (Audio|PlaySoundatLocation "/Game/G_Hall_files/Blueprints/loud_cabinet_sound.loud_cabinet_sound" (.location _returnvalue) (.rotation _returnvalue) 1.0 1.0 0.0 0 0 0))))))

(event OnComponentBeginOverlap(Box1)
  (params (OverlappedComponent :type Primitive%20Component%20Object%20Reference) (OtherActor :type Actor%20Object%20Reference) (OtherComp :type Primitive%20Component%20Object%20Reference) (OtherBodyIndex :type Integer) (bFromSweep :type Boolean) (SweepResult :type Hit%20Result%20Structure%20%28by%20ref%29))
  (bind _door (Variables|Default|GetDoor))
  ;[1 1 1] Comment
  (bind _bisheld (Class|GrippableStaticMeshComponent|IsHeld _door))
  (if _bisheld
    (Class|PrimitiveComponent|SetPhysicsMaxAngularVelocityinRadians _door 1.570796 false "None")
    (Class|GrippableStaticMeshComponent|SimulateonDrop _door)
    (else
      (Class|PrimitiveComponent|SetPhysicsAngularVelocityinDegrees _door "0, 0, 0" false "None")
      (Class|PrimitiveComponent|SetPhysicsMaxAngularVelocityinRadians _door 0.0 false "None")
      (Class|GrippableStaticMeshComponent|SimulateonDrop _door))))

(fn ConstructionScript)

(fn AdvancedGripSettings
  (return ""))

(fn ClosestGripSlotinRange
  (params (WorldLocation :type Vector :default "0, 0, 0") (bSecondarySlot :type Boolean) (CallingController :type Grip%20Motion%20Controller%20Component%20Object%20Reference) (OverridePrefix :type Name :default "None"))
  (return false ""))

(fn DenyGripping
  (return true))

(fn GetGripStiffnessandDamping
  (return 0.0 0.0))

(fn GetPrimaryGripType
  (params (bIsSlot :type Boolean))
  (return "InteractiveCollisionWithPhysics"))

(fn GripBreakDistance
  (return 0.0))

(fn GripLateUpdateSetting
  (return "LateUpdatesAlwaysOn"))

(fn GripMovementReplicationType
  (return "KeepOriginalMovement"))

(fn IsHeld
  (return 0 false))

(fn RequestsSocketing
  (return 0 "None" "" false))

(fn SecondaryGripType
  (return "SG_None"))

(fn SimulateonDrop
  (return false))

(fn TeleportBehavior
  (return "TeleportAllComponents"))